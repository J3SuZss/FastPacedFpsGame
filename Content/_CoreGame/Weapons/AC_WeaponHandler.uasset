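; Weapon handler component for BP_FirstPersonCharacter that manages equipping, firing and reloading, with a debug R key toggling the shotgun.
; EquipWeapon loads stats from DT_WeaponData, always spawns BP_Shotgun on the hand socket and links its anim layer.
; IA_Shoot spends ammo, plays a montage and camera shake without hit detection, then auto-reloads an empty magazine if reserves cover a full one.
; Fire, Reload, SwitchWeapon and GetWeaponMesh functions are empty stubs.
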(event Custom|CE_Fire
  (if (Math|Boolean|ANDBoolean (Variables|Default|GetWeaponEquipped?) (> (Variables|Default|GetCurrentAmmo) 0) (Variables|Default|GetCanFire?))
    (Math|Integer|DecrementInt (Variables|Default|GetCurrentAmmo)
      (:%20%20
        (Animation|Montage|PlayMontage (Variables|Default|GetSkeletal%20Mesh) (.firemontage (Variables|Default|GetCurrentWeaponData)) 2.0
          (:then
            (Camera|PlayWorldCameraShake "/Game/_CoreGame/Camera/Shake/BP_CameraShake.BP_CameraShake_C" (Transformation|GetWorldLocation (Variables|/Script/Engine.Actor|GetRootComponent (Variables|Default|GetOwnerChar))) 0.0 1e+03))
          (:OnCompleted
            (CallFunction|CEReload)))))))

(event Custom|CE_Reload
  (bind _currentweapondata (Variables|Default|GetCurrentWeaponData))
  (if (and (== (Variables|Default|GetCurrentAmmo) 0) (> (Variables|Default|GetTotalAmmo) 0))
    (Variables|Default|SetCanFire? false)
    (Animation|Montage|PlayMontage (Variables|Default|GetSkeletal%20Mesh) (.reloadmontage _currentweapondata)
      (:then
        (if (>= (Variables|Default|GetTotalAmmo) (.magazinesize _currentweapondata))
          (Variables|Default|SetTotalAmmo (- (Variables|Default|GetTotalAmmo) (.magazinesize _currentweapondata)))
          (Variables|Default|SetCurrentAmmo (.magazinesize _currentweapondata))))
      (:OnCompleted
        (Variables|Default|SetCanFire? true)))))

(event Input|EnhancedActionEvents|EnhancedInputActionIA_Shoot
  (params (ActionValue :type Boolean) (ElapsedSeconds :type Float%20%28double-precision%29) (TriggeredSeconds :type Float%20%28double-precision%29) (InputAction :type Input%20Action%20Object%20Reference :default "/Game/Variant_Shooter/Input/Actions/IA_Shoot.IA_Shoot"))
  (:Started
    (CallFunction|CEFire)))

(event EventBeginPlay
  (bind _asbp_first_person_character (Utilities|Casting|CastToBP_FirstPersonCharacter (Components|GetOwner)))
  (Variables|Default|SetOwnerChar _asbp_first_person_character)
  (Variables|Default|SetDT_WeaponData "/Game/_CoreGame/Weapons/WeaponData/DT_WeaponData.DT_WeaponData")
  (Variables|Default|SetSkeletal%20Mesh (Variables|/Game/_CoreGame/_MainChar/BP_FirstPersonCharacter.BP_FirstPersonCharacter_C|GetSkeletalMesh _asbp_first_person_character)))

(event Input|KeyboardEvents|DebugKeyR
  (params (Key :type Key%20Structure :default "None") (ActionValue :type Input%20Action%20Value%20Structure))
  (:Pressed
    (Utilities|FlowControl|FlipFlop
      (:A
        (CallFunction|EquipWeapon "Row_Shotgun"))
      (:B
        (CallFunction|UnequipWeapon)))))

(fn EquipWeapon
  (params (WeaponRowName :type Name))
  (bind _ownerchar (Variables|Default|GetOwnerChar))
  (bind _skeletalmesh (Variables|/Game/_CoreGame/_MainChar/BP_FirstPersonCharacter.BP_FirstPersonCharacter_C|GetSkeletalMesh _ownerchar))
  (Utilities|FlowControl|Sequence
    (:then_0
      (Utilities|IsValid (Variables|Default|GetCurrentWeapon)
        (:Is%20Valid
          (Actor|DestroyActor (Variables|Default|GetCurrentWeapon))
          (Variables|Default|SetWeaponEquipped? false))))
    (:then_1
      (bind _returnvalue (Utilities|GetDataTableRow (Variables|Default|GetDT_WeaponData) WeaponRowName)
        (:then
          (Variables|Default|SetCurrentWeaponData _returnvalue))))
    (:then_2
      (bind _returnvalue_2 (Game|SpawnActorfromClass "/Game/_CoreGame/Weapons/Shotgun/BP_Shotgun.BP_Shotgun_C" (Math|Transform|MakeTransform "0, 0, 0" "0, 0, 0" "1.000000,1.000000,1.000000") "Undefined" "MultiplyWithRoot" _ownerchar 0))
      (bind _output_get (Variables|Default|SetCurrentWeapon _returnvalue_2))
      (bind _returnvalue_3 (Transformation|AttachComponentToComponent _output_get _skeletalmesh "HandGrip_R" "KeepRelative" "KeepRelative" "KeepRelative" true))
      (Variables|Default|SetWeaponEquipped? _returnvalue_3)
      (Components|SkeletalMesh|AnimationBlueprintLinking|LinkAnimClassLayers _skeletalmesh (.WeaponAnimLayer (Utilities|Struct|BreakS_Weapons (Variables|Default|GetCurrentWeaponData)))))
    (:then_3
      (Variables|Default|SetCurrentAmmo (.MagazineSize (Utilities|Struct|BreakS_Weapons (Variables|Default|GetCurrentWeaponData))))
      (Variables|Default|SetTotalAmmo (.MaxAmmo (Utilities|Struct|BreakS_Weapons (Variables|Default|GetCurrentWeaponData)))))))

(fn UnequipWeapon
  (bind _currentweapon (Variables|Default|GetCurrentWeapon))
  (Utilities|IsValid _currentweapon
    (:Is%20Valid
      (Actor|DestroyActor _currentweapon)
      (Variables|Default|SetWeaponEquipped? false))))

(fn Fire)

(fn Reload)

(fn SwitchWeapon)

(fn GetWeaponMesh
  (return))