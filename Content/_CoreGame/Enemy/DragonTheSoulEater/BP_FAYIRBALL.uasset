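; Fireball actor for the Soul Eater dragon enemy that explodes on contact.
; Its sphere overlap ignores other fireballs and the Soul Eater, and a DoOnce limits it to one explosion.
; A hit spawns a Niagara explosion at the mesh, then timed delays hide the mesh and effect before destroying the explosion and actor.
; The graph applies no damage or movement.
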(event OnComponentBeginOverlap(Sphere)
  (params (OverlappedComponent :type Primitive%20Component%20Object%20Reference) (OtherActor :type Actor%20Object%20Reference) (OtherComp :type Primitive%20Component%20Object%20Reference) (OtherBodyIndex :type Integer) (bFromSweep :type Boolean) (SweepResult :type Hit%20Result%20Structure%20%28by%20ref%29))
  (bind _returnvalue (Utilities|GetClass OtherActor))
  (if (and (!= _returnvalue "BP_FAYIRBALL_C") (!= _returnvalue "/Game/_CoreGame/Enemy/DragonTheSoulEater/_BP_SoulEater._BP_SoulEater_C"))
    (Utilities|FlowControl|DoOnce false
      (:Completed
        (bind _returnvalue_2 (Niagara|SpawnSystematLocation "/Game/MsvFx_Niagara_Explosion_Pack_01/Prefabs/Niagara_Explosion_04.Niagara_Explosion_04" (Transformation|GetWorldLocation (Variables|Default|GetStaticMesh)) "0, 0, 0" "1.000000,1.000000,1.000000" false))
        (Utilities|FlowControl|Delay 2.0)
        (Rendering|SetVisibility (Variables|Default|GetStaticMesh) false false)
        (Rendering|SetVisibility (Variables|Default|GetNiagara) false false)
        (Utilities|FlowControl|Delay 2.0)
        (Components|DestroyComponent _returnvalue_2)
        (Actor|DestroyActor)))))

(event EventBeginPlay)

(event EventTick
  (params (DeltaSeconds :type Float%20%28single-precision%29)))

(fn ConstructionScript)