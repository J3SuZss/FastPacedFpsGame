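; Enemy spawner actor that populates the level with enemies around the player.
; On BeginPlay it caches the first-person player character and starts a fast looping timer.
; Each tick of the timer spawns a random class from EnemyTypes at a random navigable point within a radius of the player's mesh, until SpawnedEnemyCount reaches EnemyNumberThreshold.
; The count only increments, so the threshold caps total spawns rather than living enemies.
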(event Custom|CE_SpawnEnemy
  (if (> (Variables|Default|GetEnemyNumberThreshold) (Variables|Default|GetSpawnedEnemyCount))
    (bind _randomlocation (Class|NavigationSystemV1|GetRandomLocationinNavigableRadius (Transformation|GetWorldLocation (Variables|/Script/Engine.Character|GetMesh (Variables|Default|GetAs%20BP%20First%20Person%20Character))) 3e+03 0 0))
    (Game|SpawnActorfromClass (.OutItem (Utilities|Array|Random (Variables|Default|GetEnemyTypes))) (Math|Transform|MakeTransform _randomlocation "0, 0, 0" "1.000000,1.000000,1.000000") "Undefined" "MultiplyWithRoot" 0 0)
    (Math|Integer|IncrementInt (Variables|Default|GetSpawnedEnemyCount))))

(event EventBeginPlay
  (bind _asbp_first_person_character (Utilities|Casting|CastToBP_FirstPersonCharacter (Game|GetPlayerCharacter 0)))
  (Variables|Default|SetAs%20BP%20First%20Person%20Character _asbp_first_person_character)
  (Utilities|Time|SetTimerbyEvent (delegate Custom|CE_SpawnEnemy) 0.1 true))

(fn ConstructionScript)